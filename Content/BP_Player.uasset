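; Player Blueprint that grabs and manipulates objects and activates action-based dungeon event triggers by holding Interact.
; Enhanced Input actions drive a Grabber component for grab, release, rotation mode, yaw/pitch rotation and hold distance.
; Overlapping an actor with an unfinished, inactive ActionBased DungeonEventTriggerComponent stores it and shows a PlayerUI prompt.
; Tick accumulates hold time while Interact is held, then activates the event and hides the prompt.
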(event `self.ReceiveBeginPlay`
  (bind _returnvalue (`|CreateWidget` "/Game/PlayerUI.PlayerUI_C" (`GameplayStatics.GetPlayerController` 0)))
  (bind _output_get (set `self.PlayerUI` _returnvalue))
  (`UserWidget.AddToViewport` _output_get 0))

(event `self.ReceiveTick`
  (params (DeltaSeconds :type "Float (single-precision)"))
  (if (and (`self.InActionBasedTrigger`) (`self.Interact`))
    (`/Engine/EditorBlueprintResources/StandardMacros.IsValid` (`self.CurrentActionBasedTrigger`)
      (:`Is Valid`
        (set `self.CurrentHoldTime` (+ (`self.CurrentHoldTime`) DeltaSeconds))
        (if (>= (`self.CurrentHoldTime`) (`self.HoldTime`))
          (set `self.CurrentHoldTime` 0.0)
          (`DungeonEventTriggerComponent.SetDungeonEventIsActive` (`self.CurrentActionBasedTrigger`) true)
          (set `self.CurrentActionBasedTrigger` null)
          (`/Game/PlayerUI.SetVisibilityActionText` (`self.PlayerUI`) false))))
    (else
      (set `self.CurrentHoldTime` 0.0))))

(event `EnhancedInput|/Game/IA_Grab`
  (params (ActionValue :type Boolean) (ElapsedSeconds :type "Float (double-precision)") (TriggeredSeconds :type "Float (double-precision)") (InputAction :type "InputAction Object Reference" :default "/Game/IA_Grab.IA_Grab"))
  (bind _grabber (`self.Grabber`))
  (:`Started`
    (`Grabber.Grab` _grabber))
  (:`Completed`
    (`Grabber.Release` _grabber)))

(event `EnhancedInput|/Game/IA_RotationMode`
  (params (ActionValue :type Boolean) (ElapsedSeconds :type "Float (double-precision)") (TriggeredSeconds :type "Float (double-precision)") (InputAction :type "InputAction Object Reference" :default "/Game/IA_RotationMode.IA_RotationMode"))
  (bind _grabber (`self.Grabber`))
  (:`Started`
    (`Grabber.SetRotationMode` _grabber true))
  (:`Completed`
    (`Grabber.SetRotationMode` _grabber false)))

(event `EnhancedInput|/Game/IA_RotateObject`
  (params (ActionValue :type "Vector2D Structure") (ElapsedSeconds :type "Float (double-precision)") (TriggeredSeconds :type "Float (double-precision)") (InputAction :type "InputAction Object Reference" :default "/Game/IA_RotateObject.IA_RotateObject"))
  (bind (_x _y) (`KismetMathLibrary.BreakVector2D` ActionValue))
  (bind _grabber (`self.Grabber`))
  (:`Triggered`
    (`Grabber.RotateYaw` _grabber _x)
    (`Grabber.RotatePitch` _grabber _y)))

(event `EnhancedInput|/Game/IA_AdjustHoldDistance`
  (params (ActionValue :type "Float (double-precision)") (ElapsedSeconds :type "Float (double-precision)") (TriggeredSeconds :type "Float (double-precision)") (InputAction :type "InputAction Object Reference" :default "/Game/IA_AdjustHoldDistance.IA_AdjustHoldDistance"))
  (:`Triggered`
    (`Grabber.AdjustHoldDistance` (`self.Grabber`) ActionValue)))

(event `EnhancedInput|/Game/IA_Interact`
  (params (ActionValue :type Boolean) (ElapsedSeconds :type "Float (double-precision)") (TriggeredSeconds :type "Float (double-precision)") (InputAction :type "InputAction Object Reference" :default "/Game/IA_Interact.IA_Interact"))
  (:`Started`
    (set `self.Interact` true))
  (:`Completed`
    (set `self.Interact` false)))

(event `self.ReceiveActorBeginOverlap`
  (params (OtherActor :type "Actor Object Reference"))
  (bind (_returnvalue _trigger) (`self.CheckIfActionBasedTrigger` OtherActor))
  (if _returnvalue
    (if (and (not (`DungeonEventTriggerComponent.GetDungeonEventHasCompleted` _trigger)) (not (`DungeonEventTriggerComponent.GetDungeonEventIsActive` _trigger)))
      (set `self.InActionBasedTrigger` true)
      (set `self.CurrentActionBasedTrigger` _trigger)
      (`/Game/PlayerUI.SetVisibilityActionText` (`self.PlayerUI`) true))))

(event `self.ReceiveActorEndOverlap`
  (params (OtherActor :type "Actor Object Reference"))
  (if (`self.CheckIfActionBasedTrigger` OtherActor)
    (set `self.InActionBasedTrigger` false)
    (set `self.CurrentActionBasedTrigger` null)
    (`/Game/PlayerUI.SetVisibilityActionText` (`self.PlayerUI`) false)))

(fn `CheckIfActionBasedTrigger`
  (params (actor :type "Actor Object Reference"))
  (returns (ReturnValue :type Boolean) (Trigger :type "DungeonEventTriggerComponent Object Reference"))
  (bind _returnvalue (`self.GetComponentByClass` actor "/Script/CryptRaider.DungeonEventTriggerComponent"))
  (`/Engine/EditorBlueprintResources/StandardMacros.IsValid` _returnvalue
    (:`Is Valid`
      (bind _returnvalue_2 (`DungeonEventTriggerComponent.GetDungeonEventTriggerType` _returnvalue))
      (return (`|EnumEquality` _returnvalue_2 "ActionBased") _returnvalue))
    (:`Is Not Valid`
      (return false null))))

(fn `UserConstructionScript`
  (`parent.UserConstructionScript`))